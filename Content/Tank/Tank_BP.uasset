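; Player-controlled tank pawn that routes input to its movement and aiming components.
; On BeginPlay it hands the turret and barrel to TankAiming and both tracks to TankMovement.
; Move and turn axes feed TankMovement intents, aim axes rotate an azimuth gimbal and spring arm, and Fire calls TankAiming.
; The construction script assigns the turret and barrel meshes.
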(event `self.ReceiveBeginPlay`
  (`TankAimingComponent.Initialise` (`self.TankAiming`) (`self.Barrel`) (`self.turret`))
  (`TankMovementComponent.Initialise` (`self.TankMovement`) (`self.LeftTrack`) (`self.RightTrack`)))

(event `InputAxis|MoveForward`
  (params (AxisValue :type "Float (single-precision)"))
  ;[1 1 1] Movement Input Binding
  (`TankMovementComponent.IntendedMoveForward` (`self.TankMovement`) AxisValue))

(event `InputAxis|AimAzimuth`
  (params (AxisValue :type "Float (single-precision)"))
  ;[1 1 1] Balistics Input Biding
  (`SceneComponent.K2_AddLocalRotation` (`self.Azimuth Gimbal`) (`KismetMathLibrary.MakeRotator` 0.0 0.0 (* AxisValue 1.0)) false false))

(event `InputAxis|TurnRight`
  (params (AxisValue :type "Float (single-precision)"))
  ;[1 1 1] Movement Input Binding
  (`TankMovementComponent.IntendedTurnRight` (`self.TankMovement`) AxisValue))

(event `InputAxis|AimElevation`
  (params (AxisValue :type "Float (single-precision)"))
  ;[1 1 1] Balistics Input Biding
  (`SceneComponent.K2_AddLocalRotation` (`self.SpringArm1`) (`KismetMathLibrary.MakeRotator` 0.0 (* AxisValue 1.0)) false false))

(event `InputAction|Fire`
  (params (Key :type "Key Structure"))
  ;[1 1 1] Balistics Input Biding
  (:`Pressed`
    (`TankAimingComponent.Fire` (`self.TankAiming`))))

(fn `UserConstructionScript`
  (`StaticMeshComponent.SetStaticMesh` (`self.Turret`) "/Game/Tank/tank_fbx_Turret.tank_fbx_Turret")
  (`StaticMeshComponent.SetStaticMesh` (`self.Barrel`) "/Game/Tank/tank_fbx_Barrel_01.tank_fbx_Barrel_01"))